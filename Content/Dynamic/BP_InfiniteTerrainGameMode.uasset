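; Game mode for an infinite terrain game that spawns the starting tiles and keeps a score of conquered tiles.
; On BeginPlay it fills a NavMesh bounds volume pool, then spawns a few BP_Tile actors in a chain.
; Each tile receives the shared pool and supplies its attach location as the next tile's spawn transform.
; NewTileConquered increments the score, which GetScore exposes.
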(event `self.ReceiveBeginPlay`
  (`self.PopulateBoundsVolumePool`)
  (for _ (range 4)
    (`self.Spawn Tile`)))

(fn `GetScore`
  (returns (Score :type Integer))
  (return (`self.Score`)))

(fn `NewTileConquered`
  (`/Engine/EditorBlueprintResources/StandardMacros.IncrementInt` (`self.Score`)))

(fn `Spawn Tile`
  (bind _returnvalue (`|SpawnActorFromClass` "/Game/Dynamic/Terrain/BP_Tile.BP_Tile_C" (`self.nextTileTransform`) "Undefined" "OverrideRootScale" null null))
  (`Tile.SetPool` _returnvalue (`self.NavMeshBoundsVolumePool`))
  (set `self.nextTileTransform` (`/Game/Dynamic/Terrain/BP_Tile.Get Attach Location` _returnvalue)))

(fn `UserConstructionScript`)